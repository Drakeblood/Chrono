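; BP_Button is a single clickable key for the Level 1 pinpad.
; The construction script shows its NoText value on the ButtonNo text component.
; Clicking the Button component passes that value, plus confirm and backspace flags, to the referenced keypad actor through ButtonEntered.
; A ResetButtons event sets the button's material to M_Pinpad.
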(event OnClicked(Button)
  (params (TouchedComponent :type Primitive%20Component%20Object%20Reference) (ButtonPressed :type Key%20Structure))
  (Default|ButtonEntered (Variables|Default|GetKeypadActorRef) (Variables|Default|GetNoText) (Variables|Default|GetConfirm%20Button?) (Variables|Default|GetBackspace%20Button?)))

(event Custom|Reset%20Buttons
  (Rendering|Material|SetMaterial (Variables|Default|GetButton) 0 "/Game/Props/Pinpad/M_Pinpad.M_Pinpad"))

(fn ConstructionScript
  (Rendering|Components|TextRender|SetText (Variables|Default|GetButtonNo) (Variables|Default|GetNoText)))