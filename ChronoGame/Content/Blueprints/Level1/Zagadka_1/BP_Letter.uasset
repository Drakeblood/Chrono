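; BP_Letter is a readable letter for the Level 1 first puzzle (Zagadka_1).
; When the player enters its Box, it registers itself as Letter1 on BP_FirstPersonCharacter.
; LetterRead toggles the BPW_Letter1 widget on and off screen, tracked by IsReading.
; Leaving the Box clears the character's KeypadInteractActor rather than Letter1, so the letter reference remains set.
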(event OnComponentBeginOverlap(Box)
  (params (OverlappedComponent :type Primitive%20Component%20Object%20Reference) (OtherActor :type Actor%20Object%20Reference) (OtherComp :type Primitive%20Component%20Object%20Reference) (OtherBodyIndex :type Integer) (bFromSweep :type Boolean) (SweepResult :type Hit%20Result%20Structure%20%28by%20ref%29))
  (if (== OtherActor (Game|Player|GetPlayerPawn 0))
    (bind _asbp_first_person_character (Utilities|Casting|CastToBP_FirstPersonCharacter OtherActor))
    (Variables|/Game/FirstPerson/Blueprints/BP_FirstPersonCharacter.BP_FirstPersonCharacter_C|SetLetter1 _asbp_first_person_character self)))

(event OnComponentEndOverlap(Box)
  (params (OverlappedComponent :type Primitive%20Component%20Object%20Reference) (OtherActor :type Actor%20Object%20Reference) (OtherComp :type Primitive%20Component%20Object%20Reference) (OtherBodyIndex :type Integer))
  (if (== OtherActor (Game|Player|GetPlayerPawn 0))
    (bind _asbp_first_person_character (Utilities|Casting|CastToBP_FirstPersonCharacter OtherActor))
    (Variables|/Game/FirstPerson/Blueprints/BP_FirstPersonCharacter.BP_FirstPersonCharacter_C|SetKeypadInteractActor _asbp_first_person_character 0)
    (Variables|Default|SetPlayerRef 0)))

(event Custom|PutDownNote
  (Widget|RemovefromParent (stale Custom|PickupNote _returnvalue))
  (Variables|Default|SetIsReading? false))

(event Custom|TogglePickup
  (if (Variables|Default|GetIsReading?)
    (CallFunction|PutDownNote)
    (else
      (CallFunction|PickupNote))))

(event Custom|PickupNote
  (bind _returnvalue (UserInterface|CreateWidget "/Game/Blueprints/Level1/Zagadka_1/BPW_Letter1.BPW_Letter1_C"))
  (UserInterface|Viewport|AddtoViewport _returnvalue 0)
  (Variables|Default|SetIsReading? true))

(event EventLetterRead
  (CallFunction|TogglePickup))

(fn ConstructionScript)