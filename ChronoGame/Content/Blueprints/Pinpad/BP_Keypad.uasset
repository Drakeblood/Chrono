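; Keypad actor that switches the player's view to a close-up for clickable passcode entry and notifies a target actor when solved.
; Box overlap registers it with the first-person character; interaction enables the cursor and links child-actor BP_Buttons back to it.
; Button input edits a text render display masked to code length.
; Confirming compares strings: success restores the view, removes the trigger and messages KeypadTarget, while failure resets after a delay.
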(event OnComponentBeginOverlap(CollisionBox)
  (params (OverlappedComponent :type Primitive%20Component%20Object%20Reference) (OtherActor :type Actor%20Object%20Reference) (OtherComp :type Primitive%20Component%20Object%20Reference) (OtherBodyIndex :type Integer) (bFromSweep :type Boolean) (SweepResult :type Hit%20Result%20Structure%20%28by%20ref%29))
  (if (== OtherActor (Game|Player|GetPlayerPawn 0))
    (bind _asbp_first_person_character (Utilities|Casting|CastToBP_FirstPersonCharacter OtherActor))
    (Variables|/Game/FirstPerson/Blueprints/BP_FirstPersonCharacter.BP_FirstPersonCharacter_C|SetKeypadInteractActor _asbp_first_person_character self)
    (Variables|Default|SetPlayerRef _asbp_first_person_character)))

(event OnComponentEndOverlap(CollisionBox)
  (params (OverlappedComponent :type Primitive%20Component%20Object%20Reference) (OtherActor :type Actor%20Object%20Reference) (OtherComp :type Primitive%20Component%20Object%20Reference) (OtherBodyIndex :type Integer))
  (if (== OtherActor (Game|Player|GetPlayerPawn 0))
    (bind _asbp_first_person_character (Utilities|Casting|CastToBP_FirstPersonCharacter OtherActor))
    (Variables|/Game/FirstPerson/Blueprints/BP_FirstPersonCharacter.BP_FirstPersonCharacter_C|SetKeypadInteractActor _asbp_first_person_character 0)
    (Variables|Default|SetPlayerRef 0)))

(event Custom|On%20Interacted
  (bind _returnvalue (Game|GetPlayerController 0))
  (bind _enteredcodetext (Variables|Default|GetEnteredCodeText))
  (Game|Player|SetViewTargetwithBlend (Game|GetPlayerController 0) (Components|GetOwner (Variables|Default|GetCamera)) 0.4 "VTBlend_Linear" 0.0 false)
  (bind _output_get (Variables|/Script/Engine.PlayerController|SetbShowMouseCursor _returnvalue true))
  (bind _output_get_2 (Variables|/Script/Engine.PlayerController|SetbEnableClickEvents _returnvalue _output_get))
  (Variables|/Script/Engine.PlayerController|SetbEnableMouseOverEvents _returnvalue _output_get_2)
  (Rendering|Components|TextRender|SetText _enteredcodetext (Utilities|Text|MakeLiteralText (Utilities|Text|ToText(String) (Utilities|String|GetSubstring (Utilities|String|MakeLiteralString "-------") 0 (Utilities|String|Len (Variables|Default|GetKeypadCode))))))
  (Rendering|Components|TextRender|SetTextRenderColor _enteredcodetext (Math|Color|MakeColor 200 200 200 255))
  (bind _output_get_3 (Variables|Default|SetButtonsArray (Utilities|Array|MakeArray (Variables|Default|GetBPC_Button1) (Variables|Default|GetBPC_Button2) (Variables|Default|GetBPC_Button3) (Variables|Default|GetBPC_Button4) (Variables|Default|GetBPC_Button5) (Variables|Default|GetBPC_Button6) (Variables|Default|GetBPC_Button7) (Variables|Default|GetBPC_Button8) (Variables|Default|GetBPC_Button9) (Variables|Default|GetBPC_Confirm))))
  (for _array_element _output_get_3
    (bind _asbp_button (Utilities|Casting|CastToBP_Button (Variables|/Script/Engine.ChildActorComponent|GetChildActor _array_element)))
    (Variables|/Game/Blueprints/Pinpad/BP_Button.BP_Button_C|SetKeypadActorRef _asbp_button self)))

(event Custom|Initiate
  (bind _returnvalue (Game|GetPlayerController 0))
  (bind _enteredcodetext (Variables|Default|GetEnteredCodeText))
  (bind _output_get (Variables|/Script/Engine.PlayerController|SetbShowMouseCursor _returnvalue true))
  (bind _output_get_2 (Variables|/Script/Engine.PlayerController|SetbEnableClickEvents _returnvalue _output_get))
  (Variables|/Script/Engine.PlayerController|SetbEnableMouseOverEvents _returnvalue _output_get_2)
  (Rendering|Components|TextRender|SetText _enteredcodetext (Utilities|Text|MakeLiteralText (Utilities|Text|ToText(String) (Utilities|String|GetSubstring (Utilities|String|MakeLiteralString "-------") 0 (Utilities|String|Len (Variables|Default|GetKeypadCode))))))
  (Rendering|Components|TextRender|SetTextRenderColor _enteredcodetext (Math|Color|MakeColor 200 200 200 255))
  (bind _output_get_3 (Variables|Default|SetButtonsArray (Utilities|Array|MakeArray (Variables|Default|GetBPC_Button1) (Variables|Default|GetBPC_Button2) (Variables|Default|GetBPC_Button3) (Variables|Default|GetBPC_Button4) (Variables|Default|GetBPC_Button5) (Variables|Default|GetBPC_Button6) (Variables|Default|GetBPC_Button7) (Variables|Default|GetBPC_Button8) (Variables|Default|GetBPC_Button9) (Variables|Default|GetBPC_Confirm))))
  (for _array_element _output_get_3
    (bind _asbp_button (Utilities|Casting|CastToBP_Button (Variables|/Script/Engine.ChildActorComponent|GetChildActor _array_element)))
    (Variables|/Game/Blueprints/Pinpad/BP_Button.BP_Button_C|SetKeypadActorRef _asbp_button self)))

(event Custom|ButtonEntered
  (params (Value :type Text) (Confirmed? :type Boolean) (Backspace :type Boolean))
  (bind _enteredcodetext (Variables|Default|GetEnteredCodeText))
  (if Confirmed?
    (CallFunction|OnConfirmed)
    (elif Backspace
      (CallFunction|Backspace)
      (elif (Variables|Default|GetCanEnter)
        (Audio|PlaySound2D "/Game/Blueprints/Pinpad/S_pinpad.S_pinpad" 1.0 1.0 0.0 0 0)
        (Rendering|Components|TextRender|SetText _enteredcodetext (Utilities|Text|ToText(String) (Utilities|String|Replace (Utilities|String|ToString(Text) (Variables|/Script/Engine.TextRenderComponent|GetText (Variables|Default|GetEnteredCodeText))) (Utilities|String|GetSubstring (Utilities|String|MakeLiteralString "-------") 0 (Utilities|String|Len (Variables|Default|GetKeypadCode))))))
        (Rendering|Components|TextRender|SetText _enteredcodetext (Utilities|Text|ToText(String) (Utilities|String|Append (Utilities|String|ToString(Text) (Variables|/Script/Engine.TextRenderComponent|GetText (Variables|Default|GetEnteredCodeText))) (Utilities|String|ToString(Text) Value))))
        (Rendering|Components|TextRender|SetTextRenderColor (Variables|Default|GetEnteredCodeText) (Math|Color|MakeColor 255 200 200 255))))))

(event Custom|Backspace
  (bind _enteredcodetext (Variables|Default|GetEnteredCodeText))
  (bind _text (Variables|/Script/Engine.TextRenderComponent|GetText _enteredcodetext))
  (bind _returnvalue (Utilities|String|ToString(Text) _text))
  (Rendering|Components|TextRender|SetText _enteredcodetext (Utilities|Text|ToText(String) (Utilities|String|GetSubstring _returnvalue 0 (- (Utilities|String|Len _returnvalue) 1)))))

(event Custom|On%20Confirmed
  (bind _returnvalue (Game|GetPlayerController 0))
  (bind _returnvalue_2 (Game|GetPlayerController 0))
  (if (Utilities|Enum|Equal(Enum) (Variables|Default|GetKeypadCode) (Utilities|String|ToString(Text) (Variables|/Script/Engine.TextRenderComponent|GetText (Variables|Default|GetEnteredCodeText))))
    (Utilities|FlowControl|Sequence
      (:then_0
        (Rendering|Components|TextRender|SetText (Variables|Default|GetEnteredCodeText) (Utilities|Text|MakeLiteralText "Correct passcode"))
        (Rendering|Components|TextRender|SetTextRenderColor :self (Variables|Default|GetEnteredCodeText))
        (Utilities|FlowControl|RetriggerableDelay 2.0)
        (bind _output_get (Variables|/Script/Engine.PlayerController|SetbShowMouseCursor _returnvalue_2 false))
        (bind _output_get_2 (Variables|/Script/Engine.PlayerController|SetbEnableMouseOverEvents _returnvalue_2 _output_get))
        (Variables|/Script/Engine.PlayerController|SetbEnableClickEvents _returnvalue_2 _output_get_2)
        (for _array_element (Variables|Default|GetButtonsArray)
          (bind _asbp_button (Utilities|Casting|CastToBP_Button (Variables|/Script/Engine.ChildActorComponent|GetChildActor _array_element)))
          (Default|ResetButtons _asbp_button))
        (Game|Player|SetViewTargetwithBlend (Game|GetPlayerController 0) (Components|GetOwner (Variables|/Game/FirstPerson/Blueprints/BP_FirstPersonCharacter.BP_FirstPersonCharacter_C|GetFirstPersonCamera (.AsBP%20First%20Person%20Character (Utilities|Casting|CastToBP_FirstPersonCharacter (Game|Player|GetPlayerPawn 0))))) 0.4 "VTBlend_Linear" 0.0 false)
        (Rendering|Components|TextRender|SetText (Variables|Default|GetEnteredCodeText) (Utilities|Text|MakeLiteralText ""))
        (Input|SetInputModeGameOnly (Game|GetPlayerController 0) false)
        (Components|DestroyComponent (Variables|Default|GetCollisionBox))
        (Class|BPIKeypadDoor|KeypadSuccessEvent(Message) (Variables|Default|GetKeypadTarget)))
      (:then_1
        (Variables|Default|SetCanEnter false)
        (Audio|PlaySound2D "/Game/Blueprints/Pinpad/S_correct.S_correct" 1.0 1.0 0.0 0 0)))
    (else
      (Utilities|FlowControl|Sequence
        (:then_0
          (Rendering|Components|TextRender|SetText (Variables|Default|GetEnteredCodeText) (Utilities|Text|MakeLiteralText "Incorrect passcode"))
          (Rendering|Components|TextRender|SetTextRenderColor :self (Variables|Default|GetEnteredCodeText))
          (Utilities|FlowControl|RetriggerableDelay 2.0)
          (bind _output_get_3 (Variables|/Script/Engine.PlayerController|SetbShowMouseCursor _returnvalue false))
          (bind _output_get_4 (Variables|/Script/Engine.PlayerController|SetbEnableMouseOverEvents _returnvalue _output_get_3))
          (Variables|/Script/Engine.PlayerController|SetbEnableClickEvents _returnvalue _output_get_4)
          (for _array_element_2 (Variables|Default|GetButtonsArray)
            (bind _asbp_button_2 (Utilities|Casting|CastToBP_Button (Variables|/Script/Engine.ChildActorComponent|GetChildActor _array_element_2)))
            (Default|ResetButtons _asbp_button_2))
          (CallFunction|Initiate)
          (Variables|Default|SetCanEnter true))
        (:then_1
          (Variables|Default|SetCanEnter false)
          (Audio|PlaySound2D "/Game/Blueprints/Pinpad/S_wrong.S_wrong" 1.0 1.0 0.0 0 0))))))

(fn ConstructionScript)