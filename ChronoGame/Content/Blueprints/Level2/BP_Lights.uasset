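; Level 2 light sequencer that animates the intensity of an array of lights one after another once RedLightson is called.
; After a short delay, an endless delay loop periodically restarts LightsTimeline at double speed.
; The timeline drives the current light's intensity, and on finishing it replays for the next index, resetting to the first after the last light.
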(event Custom|Loop
  (bind _lightstimeline (Variables|Default|GetLightsTimeline))
  (Components|Timeline|SetPlayRate _lightstimeline 2.0 :!label _label)
  (Components|Timeline|PlayfromStart _lightstimeline)
  (Utilities|FlowControl|Delay 5.0)
  (goto _label))

(event EventRedLightson
  (Utilities|FlowControl|Delay 3.0)
  (CallFunction|Loop))

(fn ConstructionScript)